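; Launch platform that flings the player's BP_Player pawn into the air when it hits the platform's cube.
; On hit, it flags itself in use, overrides the character's jump velocity, zeroes falling lateral friction (not restored here), and triggers a jump.
; It then launches with overriding velocity: horizontal from the arrow's forward scaled by ForwardPower, vertical from jump velocity times Power.
; The construction script draws a debug line previewing forward direction and strength.
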(event `self.Cube.OnComponentHit`
  (params (HitComponent :type "PrimitiveComponent Object Reference") (OtherActor :type "Actor Object Reference") (OtherComp :type "PrimitiveComponent Object Reference") (NormalImpulse :type "Vector Structure") (Hit :type "HitResult Structure (by ref)"))
  (bind _as_bp_player (`self.As BP Player`))
  (bind _charactermovement (`Character.CharacterMovement` _as_bp_player))
  ;[0.0706 0 0.125] Component Hit
  (if (== OtherActor (`GameplayStatics.GetPlayerPawn` 0))
    (set `self.InUse` true)
    (bind _asbp_player (cast `/Game/FastMovement/Blueprints/Player/BP_Player` OtherActor))
    (set `self.As BP Player` _asbp_player)
    (set `CharacterMovementComponent.JumpZVelocity` (`self.Jump Z Velocity`) _charactermovement)
    (set `CharacterMovementComponent.FallingLateralFriction` 0.0 _charactermovement)
    (`Character.Jump` _as_bp_player)
    (`Character.Jump` _as_bp_player)
    (`Character.LaunchCharacter` _as_bp_player (`KismetMathLibrary.MakeVector` (.x (* (`SceneComponent.GetForwardVector` (`self.Arrow`)) (`self.ForwardPower`))) (.y (* (`SceneComponent.GetForwardVector` (`self.Arrow`)) (`self.ForwardPower`))) (* (`CharacterMovementComponent.JumpZVelocity` (`Character.CharacterMovement` _as_bp_player)) (`self.Power`))) true true)))

(fn `UserConstructionScript`
  (bind _returnvalue (`self.K2_GetActorLocation`))
  (`KismetSystemLibrary.DrawDebugLine` _returnvalue (+ _returnvalue (* (`SceneComponent.GetForwardVector` (`self.Arrow`)) (`self.ForwardPower`))) (struct :`R` 1.0 :`B` 0.83417 :`A` 1.0) 1.0 2.0))