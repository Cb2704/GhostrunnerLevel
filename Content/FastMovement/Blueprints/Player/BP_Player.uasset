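; BP_Player is the fast-movement player character, which adds the main screen widget on begin play.
; Its construction script passes camera, capsule and option settings to BPPlayerMovement, which also receives landing and capsule hit events.
; Dash launches the character along its horizontal velocity and slide briefly crouches above a speed threshold, both gated by delays.
; Any damage, including from a debug key, teleports the player to the last checkpoint.
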(event OnComponentHit(CapsuleComponent)
  (params (HitComponent :type Primitive%20Component%20Object%20Reference) (OtherActor :type Actor%20Object%20Reference) (OtherComp :type Primitive%20Component%20Object%20Reference) (NormalImpulse :type Vector :default "0, 0, 0") (Hit :type Hit%20Result%20Structure%20%28by%20ref%29))
  ;[0.0706 0 0.125] Capsule Hit
  (Class|BPIPlayer|PlayerCapsuleComponentHit(Message) (Variables|Default|GetBP_PlayerMovement) Hit))

(event Input|EnhancedActionEvents|EnhancedInputActionIA_Dash
  (params (ActionValue :type Boolean) (ElapsedSeconds :type Float%20%28double-precision%29) (TriggeredSeconds :type Float%20%28double-precision%29) (InputAction :type Input%20Action%20Object%20Reference :default "/Game/FastMovement/Blueprints/Player/Input/Actions/IA_Dash.IA_Dash"))
  (bind _returnvalue (Transformation|GetVelocity))
  (bind _returnvalue_2 (* _returnvalue 8.0))
  (if (not (Variables|Default|GetisDashing))
    (Variables|Default|SetisDashing true)
    (Character|LaunchCharacter (Math|Vector|MakeVector (.x _returnvalue_2) (.y _returnvalue_2) 0.0) false false)
    (Utilities|FlowControl|Delay 1.0)
    (Variables|Default|SetisDashing false)))

(event Input|EnhancedActionEvents|EnhancedInputActionSlide
  (params (ActionValue :type Boolean) (ElapsedSeconds :type Float%20%28double-precision%29) (TriggeredSeconds :type Float%20%28double-precision%29) (InputAction :type Input%20Action%20Object%20Reference :default "/Game/FastMovement/Blueprints/Player/Input/Actions/Slide.Slide"))
  (if (> (Math|Vector|VectorLength (Transformation|GetVelocity)) 5e+02)
    (Utilities|FlowControl|DoOnce false :!label _label
      (:Completed
        (Character|Crouch)
        (Development|PrintString "Hello")
        (Utilities|FlowControl|Delay 1.0)
        (Character|UnCrouch)
        (goto _label Reset)))))

(event EventOnLanded
  (params (Hit :type Hit%20Result%20Structure%20%28by%20ref%29))
  ;[0.0706 0 0.125] On Landed
  (Class|BPIPlayer|PlayeronLanded(Message) (Variables|Default|GetBP_PlayerMovement) Hit))

(event EventBeginPlay
  ;[0.0706 0 0.125] Begin Play
  (bind _returnvalue (UserInterface|CreateWidget "/Game/FastMovement/Widgets/WBP_Main_Screen.WBP_Main_Screen_C"))
  (UserInterface|Viewport|AddtoPlayerScreen _returnvalue))

(event Game|Damage|EventAnyDamage
  (params (Damage :type Float%20%28single-precision%29) (DamageType :type Damage%20Type%20Object%20Reference) (InstigatedBy :type Controller%20Object%20Reference) (DamageCauser :type Actor%20Object%20Reference))
  (bind _last_checkpoint (Variables|Default|GetLast%20Checkpoint))
  (bind _pos (Variables|/Game/Checkpoint/BP_Checkpoint.BP_Checkpoint_C|GetPOS _last_checkpoint))
  (bind _returnvalue (Transformation|GetWorldTransform _pos))
  (Transformation|Teleport (.location _returnvalue) (.rotation _returnvalue)))

(event Input|KeyboardEvents|DebugKey1
  (params (Key :type Key%20Structure :default "None") (ActionValue :type Input%20Action%20Value%20Structure))
  (:Pressed
    (Game|Damage|ApplyDamage self 1.0 0 0)))

(fn ConstructionScript
  (bind _bp_playermovement (Variables|Default|GetBP_PlayerMovement))
  ;[0.1519 0.1561 0.2917] Event Construct
  (Variables|/Game/FastMovement/Blueprints/Player/BP_PlayerMovement.BP_PlayerMovement_C|SetPlayerCameraRelativeTransorm _bp_playermovement (Transformation|GetRelativeTransform (Variables|Default|GetCamera)))
  (Variables|/Game/FastMovement/Blueprints/Player/BP_PlayerMovement.BP_PlayerMovement_C|SetPlayerCapsuleHalfHeight _bp_playermovement (Variables|/Script/Engine.CapsuleComponent|GetCapsuleHalfHeight (Variables|Collision|GetCapsuleComponent)))
  (Variables|/Game/FastMovement/Blueprints/Player/BP_PlayerMovement.BP_PlayerMovement_C|SetStruct%20Player%20Options _bp_playermovement (Variables|Default|GetPlayerOptions)))